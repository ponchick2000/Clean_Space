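; Spaceship laser Blueprint that fires BP_LaserShot actors.
; Its Shooting event spawns one shot at the location and rotation of LaserSocket1 whenever it is called with IsShooting true.
; A forward Visibility line trace from the socket is left unconnected and never runs.
; Tick, BeginPlay, ActorBeginOverlap and the construction script are empty, with the events serving only as anchors for developer notes.
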(event `/Game/FirstPerson/Blueprints/BPI_Shooting.Shooting`
  (params (bIsShooting :type Boolean))
  (bind (_returnvalue_location _returnvalue_rotation) (`KismetMathLibrary.BreakTransform` (`SceneComponent.K2_GetComponentToWorld` (`self.LaserSocket_1`))))
  ; Воспроизведение "Ивента" стрельбы
  (if bIsShooting
    (`|SpawnActorFromClass` "/Game/Blueprints/BP_LaserShot.BP_LaserShot_C" (`KismetMathLibrary.MakeTransform` _returnvalue_location _returnvalue_rotation) "Undefined" "MultiplyWithRoot" null null)))

(fn `UserConstructionScript`)