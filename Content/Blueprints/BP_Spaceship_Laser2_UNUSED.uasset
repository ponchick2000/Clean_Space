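; BP_Spaceship_Laser2_UNUSED is the spaceship's second laser, marked unused in its name; an author note says the two lasers do not currently work simultaneously.
; Its Shooting event spawns a BP_LaserShot at the LaserSocket2 world location and rotation whenever it is called with IsShooting true.
; A forward Visibility line trace from the same socket is left unconnected and never runs, and the construction script is empty.
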(event `/Game/FirstPerson/Blueprints/BPI_Shooting.Shooting`
  (params (bIsShooting :type Boolean))
  (bind (_returnvalue_location _returnvalue_rotation) (`KismetMathLibrary.BreakTransform` (`SceneComponent.K2_GetComponentToWorld` (`self.LaserSocket_2`))))
  ; Тот же принцип инициализации, как и в лазере один (НА ДАННЫЙ МОМЕНТ ДВА ЛАЗЕРА НЕ РАБОТАЮТ ОДНОВРМЕННО)
  (if bIsShooting
    (`|SpawnActorFromClass` "/Game/Blueprints/BP_LaserShot.BP_LaserShot_C" (`KismetMathLibrary.MakeTransform` _returnvalue_location _returnvalue_rotation) "Undefined" "MultiplyWithRoot" null null)))

(fn `UserConstructionScript`)